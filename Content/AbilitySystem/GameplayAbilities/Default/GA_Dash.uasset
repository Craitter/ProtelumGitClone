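; GA_Dash is a gameplay ability that gives the avatar a short, fast dash.
; For a ProtelumCharacter it commits the ability and dashes along control-rotation yaw, keeping it horizontal; otherwise it uses the actor's forward vector without committing.
; A constant-force root motion task drives the dash, restores the velocity captured at activation on finish, then ends the ability.
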(event Ability|EventActivateAbility
  (bind _returnvalue (Ability|GetAvatarActorfromActorInfo))
  (bind _asprotelum_character (Utilities|Casting|CastToProtelumCharacter _returnvalue)
    (:then
      (Ability|CommitAbility)
      (Utilities|IsValid _asprotelum_character
        (:Is%20Valid
          (Variables|Default|SetDashDirection (Math|Rotator|GetRotationXVector (Math|Rotator|MakeRotator 0.0 0.0 (.yaw (Pawn|GetControlRotation _asprotelum_character :!class /Script/Engine.Pawn))))))
        (:Is%20Not%20Valid
          (Variables|Default|SetDashDirection (Transformation|GetActorForwardVector _returnvalue) :!label _label))))
    (:CastFailed
      (goto _label)))
  (Ability|Tasks|ApplyRootMotionConstantForce "None" (Variables|Default|GetDashDirection) 6e+03 0.2 false 0 "SetVelocity" (Transformation|GetVelocity _returnvalue)
    (:OnFinish
      (Ability|EndAbility))))

(event Ability|EventOnEndAbility
  (params (bWasCancelled :type Boolean)))