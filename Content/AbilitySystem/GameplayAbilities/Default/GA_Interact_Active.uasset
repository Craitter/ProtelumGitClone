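; Gameplay ability that runs an interaction, instant or held, on a target passed in by gameplay event.
; It validates target availability and range, then sends register, pre-interact and post-interact interface messages, with optional net syncs around a UI-timed delay.
; For timed interactions, early input release cancels and release after completion ends the ability.
; Gameplay effects track the interacting state; ending clears them and the UI and sends State.Interact.End.
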(event Ability|EventOnEndAbility
  (params (bWasCancelled :type Boolean))
  (bind _returnvalue (Subsystems|GetUISubsystem))
  (bind _interact_target (Variables|Default|GetInteract%20Target))
  (bind _returnvalue_2 (Ability|TargetData|GetHitResultfromTargetData _interact_target))
  (if bWasCancelled
    (if (and (Ability|TargetData|TargetDataHasHitResult _interact_target) (Utilities|IsValid (.hitactor _returnvalue_2)))
      (Class|ProtelumInteractable|CancelInteraction(Message) (.hitactor _returnvalue_2) (.hitcomponent _returnvalue_2))))
  (bind _returnvalue_3 (Ability|ApplyGameplayEffectToOwner "/Game/AbilitySystem/GameplayEffects/Interact/GE_Interact_Remove.GE_Interact_Remove_C"))
  (Ability|RemoveGameplayEffectFromOwnerWithHandle (Variables|Default|GetGE%20Interacting%20Handle))
  (Ability|RemoveGameplayEffectFromOwnerWithHandle _returnvalue_3)
  (Class|UISubsystem|HideInteractPrompt _returnvalue)
  (Class|UISubsystem|StopInteractionTimer _returnvalue)
  (Ability|SendGameplayEvent "(TagName=\"State.Interact.End\")" (Utilities|Struct|MakeGameplayEventData "(TagName=\"\")" 0 0 0 0 "()" "(GameplayTags=)" "(GameplayTags=)" 0.0 (Variables|Default|GetInteract%20Target))))

(event Ability|EventActivateAbilityFromEvent
  (params (EventData :type Gameplay%20Event%20Data%20Structure%20%28by%20ref%29))
  (bind _returnvalue (Ability|GetAvatarActorfromActorInfo))
  (bind _returnvalue_2 (Ability|GetAvatarActorfromActorInfo))
  (bind _returnvalue_3 (Subsystems|GetUISubsystem))
  (bind _output_get (Variables|Default|SetInteract%20Target (.targetdata EventData)))
  (bind _isvalid (CallFunction|ValidateTarget _output_get))
  (if _isvalid
    (bind _returnvalue_4 (Class|ProtelumInteractable|GetInteractionDuration(Message) (.hitactor (Ability|TargetData|GetHitResultfromTargetData (Variables|Default|GetInteract%20Target))) (.hitcomponent (Ability|TargetData|GetHitResultfromTargetData (Variables|Default|GetInteract%20Target)))))
    (bind _output_get_2 (Variables|Default|SetInteractionDuration _returnvalue_4))
    (if (> _output_get_2 0.0)
      (bind _asynctaskproxy (Ability|Tasks|WaitInputRelease false)
        (:then
          (Variables|Default|SetWait%20Input%20Release%20Task _asynctaskproxy)
          (Variables|Default|SetbIsInteracting true :!label _label)
          (bind _returnvalue_5 (Ability|ApplyGameplayEffectToOwner "/Game/AbilitySystem/GameplayEffects/Interact/GE_Interact_Add.GE_Interact_Add_C"))
          (Variables|Default|SetGE%20Interacting%20Handle _returnvalue_5)
          (Class|ProtelumInteractable|RegisterInteracter(Message) (.hitactor (Ability|TargetData|GetHitResultfromTargetData (Variables|Default|GetInteract%20Target))) (.hitcomponent (Ability|TargetData|GetHitResultfromTargetData (Variables|Default|GetInteract%20Target))) _returnvalue_2)
          (bind (_bshouldsync _type) (Class|ProtelumInteractable|GetPreInteractSyncType(Message) (.hitactor (Ability|TargetData|GetHitResultfromTargetData (Variables|Default|GetInteract%20Target))) (.hitcomponent (Ability|TargetData|GetHitResultfromTargetData (Variables|Default|GetInteract%20Target)))))
          (if _bshouldsync
            (bind _asynctaskproxy_2 (Ability|Tasks|WaitNetSync _type)
              (:then
                (Variables|Default|SetPreInteractSyncTask _asynctaskproxy_2))
              (:OnSync
                (Class|ProtelumInteractable|PreInteract(Message) (.hitactor (Ability|TargetData|GetHitResultfromTargetData (Variables|Default|GetInteract%20Target))) _returnvalue_2 (.hitcomponent (Ability|TargetData|GetHitResultfromTargetData (Variables|Default|GetInteract%20Target))) :!label _label_2)
                (if (> (Variables|Default|GetInteractionDuration) 0.0)
                  (bind _asynctaskproxy_3 (Ability|Tasks|WaitDelay (Variables|Default|GetInteractionDuration))
                    (:then
                      (Variables|Default|SetWaitDelayTask _asynctaskproxy_3)
                      (Class|UISubsystem|StartInteractionTimer _returnvalue_3 (Variables|Default|GetInteractionDuration)))
                    (:OnFinish
                      (Class|UISubsystem|StopInteractionTimer _returnvalue_3 :!label _label_3)
                      (bind (_bshouldsync_2 _type_2) (Class|ProtelumInteractable|GetPostInteractSyncType(Message) (.hitactor (Ability|TargetData|GetHitResultfromTargetData (Variables|Default|GetInteract%20Target))) (.hitcomponent (Ability|TargetData|GetHitResultfromTargetData (Variables|Default|GetInteract%20Target)))))
                      (if _bshouldsync_2
                        (bind _asynctaskproxy_4 (Ability|Tasks|WaitNetSync _type_2)
                          (:then
                            (Variables|Default|SetPostInteractSyncTask _asynctaskproxy_4))
                          (:OnSync
                            (Class|ProtelumInteractable|PostInteract(Message) (.hitactor (Ability|TargetData|GetHitResultfromTargetData (Variables|Default|GetInteract%20Target))) _returnvalue (.hitcomponent (Ability|TargetData|GetHitResultfromTargetData (Variables|Default|GetInteract%20Target))) :!label _label_4)
                            (Class|ProtelumInteractable|UnregisterInteracter(Message) (.hitactor (Ability|TargetData|GetHitResultfromTargetData (Variables|Default|GetInteract%20Target))) (.hitcomponent (Ability|TargetData|GetHitResultfromTargetData (Variables|Default|GetInteract%20Target))) _returnvalue)
                            (Class|UISubsystem|HideInteractPrompt (Subsystems|GetUISubsystem))
                            (bind _returnvalue_6 (Ability|ApplyGameplayEffectToOwner "/Game/AbilitySystem/GameplayEffects/Interact/GE_Interact_Remove.GE_Interact_Remove_C"))
                            (Ability|RemoveGameplayEffectFromOwnerWithHandle (Variables|Default|GetGE%20Interacting%20Handle))
                            (Ability|RemoveGameplayEffectFromOwnerWithHandle _returnvalue_6)
                            (Variables|Default|SetbIsInteracting false)
                            (if (not (> (Variables|Default|GetInteractionDuration) 0.0))
                              (Ability|EndAbility))))
                        (else
                          (goto _label_4)))))
                  (else
                    (goto _label_3)))))
            (else
              (goto _label_2))))
        (:OnRelease
          (if (Variables|Default|GetbIsInteracting)
            (Ability|CancelAbility)
            (else
              (Ability|EndAbility)))))
      (else
        (goto _label)))
    (else
      (Ability|CancelAbility))))

(fn ValidateTarget
  (params (TargetData :type Gameplay%20Ability%20Target%20Data%20Handle%20Structure))
  (bind _returnvalue (Ability|TargetData|GetHitResultfromTargetData TargetData))
  (bind _returnvalue_2 (Class|ProtelumInteractable|IsAvailableforInteraction(Message) (.hitactor _returnvalue) (.hitcomponent _returnvalue)))
  (return (Math|Boolean|ANDBoolean (Ability|TargetData|TargetDataHasHitResult TargetData) (== (Ability|TargetData|GetDataCountfromTargetData TargetData) 1) (Utilities|IsValid (.hitactor _returnvalue)) _returnvalue_2 (Utilities|IsValid (.hitcomponent _returnvalue)) (< (Class|KismetMathLibrary|VectorDistanceSquared (Transformation|GetActorLocation (Ability|GetAvatarActorfromActorInfo)) (Transformation|GetWorldLocation (.hitcomponent _returnvalue))) (Math|Float|Square 5e+02)))))