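; Passive interaction ability that traces for nearby interactable targets from the avatar, shows their interact prompt and waits for input.
; A press sends State.Interact.Begin with the target data once State.Interact.Block is absent, while losing the target cancels pending tasks.
; State.Interact.End re-arms input for the same component, after release if held.
; Comparing State.Interacting Add and Remove tag counts gates input and prompt hiding.
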(event Custom|Wait%20For%20Interact%20Input
  (bind _returnvalue (Ability|GetAbilitySystemComponentfromActorInfo))
  (bind _returnvalue_2 (Subsystems|GetUISubsystem))
  (bind _currenttracedtarget (Variables|Default|GetCurrentTracedTarget))
  (bind _returnvalue_3 (Ability|TargetData|GetHitResultfromTargetData _currenttracedtarget))
  ;[1 1 1] Wait for Input to Start Interactiong
  (bind _returnvalue_4 (Class|ProtelumInteractable|GetInteractionDuration(Message) (.hitactor _returnvalue_3) (.hitcomponent _returnvalue_3)))
  (Utilities|IsValid _returnvalue_2
    (:Is%20Valid
      (bind _returnvalue_5 (Class|ProtelumInteractable|GetInteractionMessageType(Message) (.hitactor _returnvalue_3) (.hitcomponent _returnvalue_3)))
      (Class|UISubsystem|ShowInteractPrompt _returnvalue_2 _returnvalue_4 _returnvalue_5)
      (if (<= (Class|AbilitySystemComponent|GetGameplayTagCount _returnvalue "(TagName=\"State.Interacting.Add\")") (Class|AbilitySystemComponent|GetGameplayTagCount _returnvalue "(TagName=\"State.Interacting.Remove\")"))
        (bind _asynctaskproxy (Ability|Tasks|WaitInputPress true)
          (:then
            (Variables|Default|SetWaitInteractInputTask _asynctaskproxy))
          (:OnPress
            (bind _asynctaskproxy_2 (Ability|Tasks|WaitGameplayTagRemove "(TagName=\"State.Interact.Block\")" 0 true)
              (:then
                (Variables|Default|SetBlockInteractRemovedTask _asynctaskproxy_2))
              (:Removed
                (bind _waitinteractinputtask (Variables|Default|GetWaitInteractInputTask)
                  (:then
                    (GameplayTasks|EndTask _waitinteractinputtask))
                  (:else
                    _))
                (Ability|SendGameplayEvent "(TagName=\"State.Interact.Begin\")" (Utilities|Struct|MakeGameplayEventData "(TagName=\"\")" 0 0 0 0 "()" "(GameplayTags=)" "(GameplayTags=)" 0.0 (Variables|Default|GetCurrentTracedTarget)))))))))))

(event Ability|EventActivateAbility
  (bind _returnvalue (Ability|GetAbilitySystemComponentfromActorInfo))
  (bind (_asynctaskproxy _data) (|WaitforInteractableTarget "None" (Utilities|Struct|MakeGameplayAbilityTargetingLocationInfo "ActorTransform" "0.000000,0.000000,0.000000|0.000000,0.000000,-0.000000|1.000000,1.000000,1.000000" (Ability|GetAvatarActorfromActorInfo) 0 self) "(Name=\"InteractTrace\")" 3e+02 0.1 false)
    (:then
      (Variables|Default|SetWaitForInteractableTarget _asynctaskproxy)
      (bind _payload (Ability|Tasks|WaitGameplayEvent "(TagName=\"State.Interact.End\")" 0)
        (:EventReceived
          (if (Math|Boolean|ANDBoolean (Math|Boolean|NANDBoolean (Utilities|IsValid (Variables|Default|GetWaitInteractInputTask)) (Utilities|IsValid (Variables|Default|GetBlockInteractRemovedTask))) (== (Ability|TargetData|GetDataCountfromTargetData (.targetdata _payload)) 1) (Ability|TargetData|TargetDataHasHitResult (.targetdata _payload)) (== (Ability|TargetData|GetDataCountfromTargetData (Variables|Default|GetCurrentTracedTarget)) 1) (Ability|TargetData|TargetDataHasHitResult (Variables|Default|GetCurrentTracedTarget)) (== (.hitcomponent (Ability|TargetData|GetHitResultfromTargetData (.targetdata _payload))) (.hitcomponent (Ability|TargetData|GetHitResultfromTargetData (Variables|Default|GetCurrentTracedTarget)))))
            (if (Class|ProtelumGameplayAbility|IsInputPressed)
              (bind _asynctaskproxy_2 (Ability|Tasks|WaitInputRelease false)
                (:then
                  (Variables|Default|SetWaitReleaseInteractInput _asynctaskproxy_2))
                (:OnRelease
                  (CallFunction|WaitforInteractInput :!label _label)))
              (else
                (goto _label)))))))
    (:FoundNewInteractableTarget
      (Variables|Default|SetCurrentTracedTarget _data)
      (CallFunction|WaitforInteractInput))
    (:LostInteractableTarget
      (bind _waitinteractinputtask (Variables|Default|GetWaitInteractInputTask)
        (:then
          (GameplayTasks|EndTask _waitinteractinputtask))
        (:else
          _))
      (bind _blockinteractremovedtask (Variables|Default|GetBlockInteractRemovedTask)
        (:then
          (GameplayTasks|EndTask _blockinteractremovedtask))
        (:else
          _))
      (bind _waitreleaseinteractinput (Variables|Default|GetWaitReleaseInteractInput)
        (:then
          (GameplayTasks|EndTask _waitreleaseinteractinput))
        (:else
          _))
      (Class|ProtelumGameplayAbility|ClearTargetData (Variables|Default|GetCurrentTracedTarget))
      (if (<= (Class|AbilitySystemComponent|GetGameplayTagCount _returnvalue "(TagName=\"State.Interacting.Add\")") (Class|AbilitySystemComponent|GetGameplayTagCount _returnvalue "(TagName=\"State.Interacting.Remove\")"))
        (Class|UISubsystem|HideInteractPrompt (Subsystems|GetUISubsystem))))))

(event Ability|EventOnEndAbility
  (params (bWasCancelled :type Boolean))
  ;[1 1 1] Wait for Input to Start Interactiong
)