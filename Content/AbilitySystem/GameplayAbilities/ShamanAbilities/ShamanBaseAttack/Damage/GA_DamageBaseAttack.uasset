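; Gameplay ability for the Shaman's damage base attack, firing a single-target projectile.
; After committing, the authority spawns BP_ShamanProjectile at the weapon socket, aimed by camera yaw only, configures it, then ends the ability.
; The projectile carries a heal-ammo regeneration effect for the instigator and a damage effect for the target, with damage set by caller from the character's projectile damage.
; A failed cast or commit cancels the ability.
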(event Ability|EventActivateAbility
  (bind _asprotelum_character (Utilities|Casting|CastToProtelumCharacter (.AvatarActor (Utilities|Struct|BreakGameplayAbilityActorInfo (Ability|GetActorInfo))))
    (:then
      (Variables|Default|SetProtelumChar _asprotelum_character)
      (bind _returnvalue (Ability|CommitAbility))
      (if _returnvalue
        (if (Ability|HasAuthority (Variables|Default|GetProtelumChar))
          (CallFunction|SetInstigatorEffects)
          (CallFunction|SetTargetEffects)
          (bind _spawntransform (CallFunction|GetSpawnTransform))
          (bind _returnvalue_2 (Game|SpawnActorfromClass "/Game/AbilitySystem/GameplayAbilities/ShamanAbilities/BP_ShamanProjectile.BP_ShamanProjectile_C" _spawntransform "Undefined" (Variables|Default|GetProtelumChar) (Variables|Default|GetProtelumChar)))
          (bind _output_get (Variables|Default|SetProjectile _returnvalue_2))
          (Utilities|IsValid _output_get
            (:Is%20Valid
              (Class|SimpleProjectile|ConfigureProjectile (Variables|Default|GetProjectile) "SingleTarget" (Variables|Default|GetInstigatorEffects) (Variables|Default|GetTargetEffects) 0.0 3e+01 (Variables|Default|GetProjectileColor) (Math|Vector|MakeVector 5e+03 0.0 0.0) false))
            (:Is%20Not%20Valid
              _))
          (Ability|EndAbility))
        (else
          (Ability|CancelAbility :!label _label))))
    (:CastFailed
      (goto _label))))

(event Ability|EventOnEndAbility
  (params (bWasCancelled :type Boolean)))

(fn GetSpawnTransform
  (bind _protelumchar (Variables|Default|GetProtelumChar))
  (return (Math|Transform|MakeTransform (Transformation|GetSocketLocation (Class|ProtelumCharacter|GetWeapon _protelumchar) "projectile") (Math|Rotator|MakeRotator 0.0 0.0 (.yaw (Transformation|GetWorldRotation (Class|ProtelumCharacter|GetCamera _protelumchar)))))))

(fn SetInstigatorEffects
  (Variables|Default|SetInstigatorEffects (Utilities|Array|MakeArray (Ability|MakeOutgoingGameplayEffectSpec "/Game/AbilitySystem/GameplayAbilities/ShamanAbilities/ShamanBaseAttack/Damage/GE_RegenerateHealAmmo.GE_RegenerateHealAmmo_C" (Math|Conversions|ToFloat(Integer) (Ability|GetAbilityLevel)))))
  (return))

(fn SetTargetEffects
  (bind _returnvalue (Ability|GameplayEffect|AssignTagSetbyCallerMagnitude (Ability|MakeOutgoingGameplayEffectSpec "/Game/AbilitySystem/GameplayEffects/GE_SimpleDamage.GE_SimpleDamage_C" (Math|Conversions|ToFloat(Integer) (Ability|GetAbilityLevel))) "(TagName=\"Data.Damage\")" (Class|ProtelumCharacterBase|GetProjectileDamage (Variables|Default|GetProtelumChar))))
  (Variables|Default|SetTargetEffects (Utilities|Array|MakeArray _returnvalue))
  (return))