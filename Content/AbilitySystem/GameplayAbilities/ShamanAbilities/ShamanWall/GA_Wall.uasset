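; Shaman gameplay ability that lets the player aim and place a wall.
; It reads wall stats from a level curve table, then configures a box preview target actor, cached on the character for reuse, with size and range.
; Confirming commits the ability and spawns BP_Shaman_Wall at the targeted transform; cancelling ends it.
; The effect that would initialize wall attributes is unwired, and Health and Cooldown are stored but unused here.
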(event Ability|EventActivateAbility
  (bind _returnvalue (Ability|GetAvatarActorfromActorInfo))
  (bind _range (Variables|Default|GetRange))
  (bind _asprotelum_character (Utilities|Casting|CastToProtelumCharacter _returnvalue))
  (CallFunction|SetUpTargetActor)
  (CallFunction|EvaluateLevelParameters)
  (Class|PGATAGroundDeploy|Configure (Variables|Default|GetTargetActor) (Utilities|Struct|MakeGameplayAbilityTargetingLocationInfo "SocketTransform" (Math|Transform|MakeTransform "0, 0, 0" "0, 0, 0" "1.000000,1.000000,1.000000") _returnvalue (Class|ProtelumCharacter|GetWeapon _asprotelum_character) self "Projectile") "(Name=\"IgnoreOnlyPawn\")" "Box" "0.000000,90.000000,0.000000" (Variables|Default|GetLength) (Variables|Default|GetHeight) (Variables|Default|GetWidth) 0.0 _range _range true true false false)
  (bind _data (|WaitTargetDataReUsingActor "None" "UserConfirmed" (Variables|Default|GetTargetActor) true)
    (:then
      (|WaitConfirmCancel
        (:OnCancel
          (Ability|EndAbility :!label _label))))
    (:ValidData
      (Ability|CommitAbility)
      (bind _returnvalue_2 (Class|ProtelumGameplayAbility|GetTargetLocationInfobyIndexOfTargetDataHandle _data))
      (bind _asprotelum_character_2 (Utilities|Casting|CastToProtelumCharacter (Ability|GetAvatarActorfromActorInfo))
        (:then
          _)
        (:CastFailed
          _))
      (bind _returnvalue_3 (Game|SpawnActorfromClass "/Game/AbilitySystem/GameplayAbilities/ShamanAbilities/ShamanWall/BP_Shaman_Wall.BP_Shaman_Wall_C" (.LiteralTransform (Utilities|Struct|BreakGameplayAbilityTargetingLocationInfo _returnvalue_2)) "AlwaysSpawn" _asprotelum_character_2 _asprotelum_character_2))
      (Ability|EndAbility))
    (:Cancelled
      (goto _label))))

(event Ability|EventOnEndAbility
  (params (bWasCancelled :type Boolean))
  (if bWasCancelled
    _))

(fn EvaluateLevelParameters
  (bind _outxy (DataTable|EvaluateCurveTableRow "/Game/AbilitySystem/GameplayAbilities/ShamanAbilities/ShamanWall/ShamanAbilityLevels_-_WallLevel.ShamanAbilityLevels_-_WallLevel" "Health" (Math|Conversions|ToFloat(Integer) (Ability|GetAbilityLevel)))
    (:RowFound
      (Variables|Default|SetHealth _outxy))
    (:RowNotFound
      _))
  (bind _outxy_2 (DataTable|EvaluateCurveTableRow "/Game/AbilitySystem/GameplayAbilities/ShamanAbilities/ShamanWall/ShamanAbilityLevels_-_WallLevel.ShamanAbilityLevels_-_WallLevel" "Height" (Math|Conversions|ToFloat(Integer) (Ability|GetAbilityLevel)))
    (:RowFound
      (Variables|Default|SetHeight _outxy_2))
    (:RowNotFound
      _))
  (bind _outxy_3 (DataTable|EvaluateCurveTableRow "/Game/AbilitySystem/GameplayAbilities/ShamanAbilities/ShamanWall/ShamanAbilityLevels_-_WallLevel.ShamanAbilityLevels_-_WallLevel" "Width" (Math|Conversions|ToFloat(Integer) (Ability|GetAbilityLevel)))
    (:RowFound
      (Variables|Default|SetWidth _outxy_3))
    (:RowNotFound
      _))
  (bind _outxy_4 (DataTable|EvaluateCurveTableRow "/Game/AbilitySystem/GameplayAbilities/ShamanAbilities/ShamanWall/ShamanAbilityLevels_-_WallLevel.ShamanAbilityLevels_-_WallLevel" "Cooldown" (Math|Conversions|ToFloat(Integer) (Ability|GetAbilityLevel)))
    (:RowFound
      (Variables|Default|SetCooldown _outxy_4))
    (:RowNotFound
      _))
  (bind _outxy_5 (DataTable|EvaluateCurveTableRow "/Game/AbilitySystem/GameplayAbilities/ShamanAbilities/ShamanWall/ShamanAbilityLevels_-_WallLevel.ShamanAbilityLevels_-_WallLevel" "Range" (Math|Conversions|ToFloat(Integer) (Ability|GetAbilityLevel)))
    (:RowFound
      (Variables|Default|SetRange _outxy_5))
    (:RowNotFound
      _))
  (bind _outxy_6 (DataTable|EvaluateCurveTableRow "/Game/AbilitySystem/GameplayAbilities/ShamanAbilities/ShamanWall/ShamanAbilityLevels_-_WallLevel.ShamanAbilityLevels_-_WallLevel" "Lenght" (Math|Conversions|ToFloat(Integer) (Ability|GetAbilityLevel)))
    (:RowFound
      (Variables|Default|SetLength _outxy_6))))

(fn SetUpTargetActor
  (bind _asprotelum_character (Utilities|Casting|CastToProtelumCharacter (Ability|GetAvatarActorfromActorInfo)))
  (bind _returnvalue (Class|ProtelumCharacter|GetTargetActorReference _asprotelum_character self "/Game/AbilitySystem/GameplayAbilities/ShamanAbilities/ShamanWall/BP_WallPreview.BP_WallPreview_C"))
  (Utilities|IsValid _returnvalue
    (:Is%20Valid
      (bind _asp_gata_ground_deploy (Utilities|Casting|CastToP_GATA_GroundDeploy _returnvalue))
      (Variables|Default|SetTargetActor _asp_gata_ground_deploy))
    (:Is%20Not%20Valid
      (bind _returnvalue_2 (Game|SpawnActorfromClass :Class "/Game/AbilitySystem/GameplayAbilities/ShamanAbilities/ShamanWall/BP_WallPreview.BP_WallPreview_C" :SpawnTransform (Variables|Default|GetLiteral%20Transform) :CollisionHandlingOverride "AlwaysSpawn" :StartLocation (Class|GameplayAbility|MakeTargetLocationInfofromOwnerActor) :ReticleClass 0 :Instigator 0))
      (bind _output_get (Variables|Default|SetTargetActor _returnvalue_2))
      (Class|ProtelumCharacter|SetTargetActorReference _asprotelum_character self _output_get))))