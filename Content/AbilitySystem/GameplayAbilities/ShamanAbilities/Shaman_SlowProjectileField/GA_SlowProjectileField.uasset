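; Shaman gameplay ability that fires a projectile for the Slow Projectile Field skill.
; After committing, the server spawns BP_ShamanProjectile at the weapon socket along camera yaw and configures its effects, lifespan and velocity.
; Confirm triggers the projectile early; confirm, cancel or projectile expiry ends the ability.
; GetLevelParameters reads lifespans, slow strength and diameter from a level curve table, while SetTargetEffects is an empty stub.
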(event Custom|OnProjectileLifeEnds_Event
  (params (ActorLocation :type Vector%20%28by%20ref%29) (bAlreadyTriggered :type Boolean))
  (Ability|EndAbility)
  (Development|PrintString "Hello"))

(event Ability|EventActivateAbility
  (bind _asprotelum_character (Utilities|Casting|CastToProtelumCharacter (.AvatarActor (Utilities|Struct|BreakGameplayAbilityActorInfo (Ability|GetActorInfo))))
    (:then
      (Variables|Default|SetProtelum%20Char _asprotelum_character)
      (bind _returnvalue (Ability|CommitAbility))
      (if _returnvalue
        (if (Ability|HasAuthority (Variables|Default|GetProtelum%20Char))
          (bind _spawntransform (CallFunction|GetSpawnTransform))
          (bind _returnvalue_2 (Game|SpawnActorfromClass "/Game/AbilitySystem/GameplayAbilities/ShamanAbilities/BP_ShamanProjectile.BP_ShamanProjectile_C" _spawntransform "Undefined" (Variables|Default|GetProtelum%20Char) (Variables|Default|GetProtelum%20Char)))
          (bind _output_get (Variables|Default|SetProjectile _returnvalue_2))
          (Utilities|IsValid _output_get
            (:Is%20Valid
              (Class|SimpleProjectile|ConfigureProjectile _output_get "SingleTarget" (Variables|Default|GetInstigator%20Effects) (Variables|Default|GetTarget%20Effects) 0.0 (Variables|Default|GetProjectile%20Life%20Span) (Variables|Default|GetProjectile%20Color) (Math|Vector|MakeVector 2e+03 0.0 0.0) false)
              (|WaitConfirmCancel
                (:then
                  (EventDispatchers|AssignOnProjectileLifeEnds (Variables|Default|GetProjectile) (delegate Custom|OnProjectileLifeEnds_Event)))
                (:OnConfirm
                  (Class|SimpleProjectile|ConfirmbyInstigator (Variables|Default|GetProjectile))
                  (Ability|EndAbility :!label _label))
                (:OnCancel
                  (goto _label))))
            (:Is%20Not%20Valid
              (goto _label))))
        (else
          (Ability|CancelAbility :!label _label_2))))
    (:CastFailed
      (goto _label_2))))

(event Ability|EventOnEndAbility
  (params (bWasCancelled :type Boolean)))

(fn GetSpawnTransform
  (bind _protelum_char (Variables|Default|GetProtelum%20Char))
  (return (Math|Transform|MakeTransform (Transformation|GetSocketLocation (Class|ProtelumCharacter|GetWeapon _protelum_char) "projectile") (Math|Rotator|MakeRotator 0.0 0.0 (.yaw (Transformation|GetWorldRotation (Class|ProtelumCharacter|GetCamera _protelum_char)))))))

(fn SetTargetEffects)

(fn GetLevelParameters
  (bind _outxy (DataTable|EvaluateCurveTableRow "/Game/AbilitySystem/GameplayAbilities/ShamanAbilities/Shaman_SlowProjectileField/ShamanAbilityLevels_-_SlowProjectileField.ShamanAbilityLevels_-_SlowProjectileField" "ProjectileLifeSpan" (Math|Conversions|ToFloat(Integer) (Ability|GetAbilityLevel)))
    (:RowFound
      (Variables|Default|SetProjectile%20Life%20Span _outxy))
    (:RowNotFound
      _))
  (bind _outxy_2 (DataTable|EvaluateCurveTableRow "/Game/AbilitySystem/GameplayAbilities/ShamanAbilities/Shaman_SlowProjectileField/ShamanAbilityLevels_-_SlowProjectileField.ShamanAbilityLevels_-_SlowProjectileField" "SlowFieldLifeSpan" (Math|Conversions|ToFloat(Integer) (Ability|GetAbilityLevel)))
    (:RowFound
      (Variables|Default|SetSlowFieldLifeSpan _outxy_2))
    (:RowNotFound
      _))
  (bind _outxy_3 (DataTable|EvaluateCurveTableRow "/Game/AbilitySystem/GameplayAbilities/ShamanAbilities/Shaman_SlowProjectileField/ShamanAbilityLevels_-_SlowProjectileField.ShamanAbilityLevels_-_SlowProjectileField" "SlowStrenght" (Math|Conversions|ToFloat(Integer) (Ability|GetAbilityLevel)))
    (:RowFound
      (Variables|Default|SetSlowStrenght _outxy_3))
    (:RowNotFound
      _))
  (bind _outxy_4 (DataTable|EvaluateCurveTableRow "/Game/AbilitySystem/GameplayAbilities/ShamanAbilities/Shaman_SlowProjectileField/ShamanAbilityLevels_-_SlowProjectileField.ShamanAbilityLevels_-_SlowProjectileField" "Diameter" (Math|Conversions|ToFloat(Integer) (Ability|GetAbilityLevel)))
    (:RowFound
      (Variables|Default|SetDiameter _outxy_4))
    (:RowNotFound
      _))
  (return))