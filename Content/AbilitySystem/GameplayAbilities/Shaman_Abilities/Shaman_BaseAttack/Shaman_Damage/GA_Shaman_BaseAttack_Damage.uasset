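; Shaman base attack gameplay ability that fires a single-target damage projectile.
; On activation it commits, then on the server spawns BP_Shaman_Projectile at the character's projectile spawn transform and ends; failed checks cancel it.
; It hands the projectile two effect lists: heal-ammo regen for the instigator, and simple damage for the target, with magnitude set by caller from the character's projectile damage.
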(event Ability|EventActivateAbility
  (bind _asprotelum_character (Utilities|Casting|CastToProtelumCharacter (Ability|GetAvatarActorfromActorInfo))
    (:then
      (bind _output_get (Variables|Default|SetProtelumChar _asprotelum_character))
      (Utilities|IsValid _output_get
        (:Is%20Valid
          (bind _returnvalue (Ability|CommitAbility))
          (if _returnvalue
            (if (Ability|HasAuthority (Variables|Default|GetProtelumChar))
              (CallFunction|SetInstigatorEffects)
              (CallFunction|SetTargetEffects)
              (bind _returnvalue_2 (Class|ProtelumCharacter|GetProjectileSpawnTransform (Variables|Default|GetProtelumChar)))
              (bind _returnvalue_3 (Game|SpawnActorfromClass "/Game/AbilitySystem/GameplayAbilities/Shaman_Abilities/BP_Shaman_Projectile.BP_Shaman_Projectile_C" _returnvalue_2 "Undefined" (Variables|Default|GetProtelumChar) (Variables|Default|GetProtelumChar)))
              (bind _output_get_2 (Variables|Default|SetProjectile _returnvalue_3))
              (Utilities|IsValid _output_get_2
                (:Is%20Valid
                  (Class|SimpleProjectile|ConfigureProjectile (Variables|Default|GetProjectile) "SingleTarget" (Variables|Default|GetInstigatorEffects) (Variables|Default|GetTargetEffects) 0.0 3e+01 (Variables|Default|GetProjectileColor) (Math|Vector|MakeVector 5e+03 0.0 0.0) false))
                (:Is%20Not%20Valid
                  _))
              (Ability|EndAbility))
            (else
              (Ability|CancelAbility :!label _label))))
        (:Is%20Not%20Valid
          (goto _label))))
    (:CastFailed
      (goto _label))))

(event Ability|EventOnEndAbility
  (params (bWasCancelled :type Boolean)))

(fn SetInstigatorEffects
  (Variables|Default|SetInstigatorEffects (Utilities|Array|MakeArray (Ability|MakeOutgoingGameplayEffectSpec "/Game/AbilitySystem/GameplayAbilities/Shaman_Abilities/Shaman_BaseAttack/Shaman_Damage/GE_Shaman_Projectile_Regen_HealAmmo.GE_Shaman_Projectile_Regen_HealAmmo_C" (Math|Conversions|ToFloat(Integer) (Ability|GetAbilityLevel)))))
  (return))

(fn SetTargetEffects
  (bind _returnvalue (Ability|GameplayEffect|AssignTagSetbyCallerMagnitude (Ability|MakeOutgoingGameplayEffectSpec "/Game/AbilitySystem/GameplayEffects/GE_SimpleDamage.GE_SimpleDamage_C" (Math|Conversions|ToFloat(Integer) (Ability|GetAbilityLevel))) "(TagName=\"Data.Damage\")" (Class|ProtelumCharacterBase|GetProjectileDamage (Variables|Default|GetProtelumChar))))
  (Variables|Default|SetTargetEffects (Utilities|Array|MakeArray _returnvalue))
  (return))