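; Shaman heal circle gameplay ability that spawns a BP_Shaman_HealCircle actor at the caster's root socket.
; GetLevelParameters reads diameter, duration, heal value and cooldown from a curve table by ability level.
; Activation commits, spawns the circle scaled by diameter with parent attachment and a level-based GE_Shaman_HealCircle spec, sets its lifespan to duration, then ends.
; Heal value and cooldown are stored but unused in these graphs.
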(event Ability|EventActivateAbility
  (bind _diameter (Variables|Default|GetDiameter))
  (Variables|Default|SetSocketName "root")
  (CallFunction|GetLevelParameters)
  (bind _asprotelum_character (Utilities|Casting|CastToProtelumCharacter (Ability|GetAvatarActorfromActorInfo))
    (:then
      (Variables|Default|SetProtelum%20Character _asprotelum_character)
      (Variables|Default|SetSpawnTransform (Math|Transform|MakeTransform (Transformation|GetSocketLocation (Variables|/Script/Engine.Character|GetMesh (Variables|Default|GetProtelum%20Character)) (Variables|Default|GetSocketName)) "0, 0, 0" (Math|Vector|MakeVector _diameter _diameter 5e+01)))
      (Ability|CommitAbility)
      (bind _returnvalue (Game|SpawnActorfromClass "/Game/AbilitySystem/GameplayAbilities/Shaman_Abilities/Shaman_HealCircle/BP_Shaman_HealCircle.BP_Shaman_HealCircle_C" (Variables|Default|GetSpawnTransform) "Undefined" 0 (Utilities|Array|MakeArray (Ability|MakeOutgoingGameplayEffectSpec "/Game/AbilitySystem/GameplayAbilities/Shaman_Abilities/Shaman_HealCircle/GE_Shaman_HealCircle.GE_Shaman_HealCircle_C" (Math|Conversions|ToFloat(Integer) (Ability|GetAbilityLevel)))) true (Variables|Default|GetSocketName) (Variables|Default|GetProtelum%20Character)))
      (Actor|SetLifeSpan _returnvalue (Variables|Default|GetDuration))
      (Ability|EndAbility))
    (:CastFailed
      (Ability|CancelAbility))))

(event Ability|EventOnEndAbility
  (params (bWasCancelled :type Boolean)))

(fn GetLevelParameters
  (bind _outxy (DataTable|EvaluateCurveTableRow "/Game/AbilitySystem/GameplayAbilities/Shaman_Abilities/Shaman_HealCircle/ShamanAbilityLevels_-_ShamanHealCircle.ShamanAbilityLevels_-_ShamanHealCircle" "Diameter" (Math|Conversions|ToFloat(Integer) (Ability|GetAbilityLevel)))
    (:RowFound
      (Variables|Default|SetDiameter _outxy))
    (:RowNotFound
      _))
  (bind _outxy_2 (DataTable|EvaluateCurveTableRow "/Game/AbilitySystem/GameplayAbilities/Shaman_Abilities/Shaman_HealCircle/ShamanAbilityLevels_-_ShamanHealCircle.ShamanAbilityLevels_-_ShamanHealCircle" "Duration" (Math|Conversions|ToFloat(Integer) (Ability|GetAbilityLevel)))
    (:RowFound
      (Variables|Default|SetDuration _outxy_2))
    (:RowNotFound
      _))
  (bind _outxy_3 (DataTable|EvaluateCurveTableRow "/Game/AbilitySystem/GameplayAbilities/Shaman_Abilities/Shaman_HealCircle/ShamanAbilityLevels_-_ShamanHealCircle.ShamanAbilityLevels_-_ShamanHealCircle" "HealValue" (Math|Conversions|ToFloat(Integer) (Ability|GetAbilityLevel)))
    (:RowFound
      (Variables|Default|SetHealValue _outxy_3))
    (:RowNotFound
      _))
  (bind _outxy_4 (DataTable|EvaluateCurveTableRow "/Game/AbilitySystem/GameplayAbilities/Shaman_Abilities/Shaman_HealCircle/ShamanAbilityLevels_-_ShamanHealCircle.ShamanAbilityLevels_-_ShamanHealCircle" "Cooldown" (Math|Conversions|ToFloat(Integer) (Ability|GetAbilityLevel)))
    (:RowFound
      (Variables|Default|SetCooldown _outxy_4))))