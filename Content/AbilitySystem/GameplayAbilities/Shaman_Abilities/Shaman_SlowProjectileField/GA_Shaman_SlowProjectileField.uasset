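; Shaman gameplay ability that fires a projectile which leaves a slow field on the ground when its life ends.
; After commit, the server spawns and configures the projectile with level-based curve table values, then waits for confirm or cancel; confirm notifies the projectile.
; On life end, a downward trace places a fixed-scale BP_Shaman_SlowField at the last hit, carrying the slow effect spec and a level-based lifespan.
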(event Custom|OnProjectileLifeEnds_Event
  (params (ActorLocation :type Vector%20%28by%20ref%29) (bAlreadyTriggered :type Boolean))
  (bind _protelum_char (Variables|Default|GetProtelum%20Char))
  (Ability|EndAbility)
  (CallFunction|SetTargetEffects)
  (bind (_outhits _returnvalue) (Class|KismetSystemLibrary|LineTraceMultibyProfile ActorLocation (- ActorLocation "0.000000,0.000000,500.000000") "Projectile" false 0 "ForDuration" true))
  (if _returnvalue
    (bind _returnvalue_2 (Game|SpawnActorfromClass "/Game/AbilitySystem/GameplayAbilities/Shaman_Abilities/Shaman_SlowProjectileField/BP_Shaman_SlowField.BP_Shaman_SlowField_C" (Math|Transform|MakeTransform (.impactpoint (Utilities|Array|Get(acopy) _outhits (Utilities|Array|LastIndex _outhits))) "0, 0, 0" (Math|Vector|MakeVector 5.0 5.0 5.0)) "AlwaysSpawn" _protelum_char (Variables|Default|GetTarget%20Effects) false "None" _protelum_char))
    (Actor|SetLifeSpan _returnvalue_2 (Variables|Default|GetSlowFieldLifeSpan))))

(event Ability|EventActivateAbility
  (bind _asprotelum_character (Utilities|Casting|CastToProtelumCharacter (Ability|GetAvatarActorfromActorInfo))
    (:then
      (bind _output_get (Variables|Default|SetProtelum%20Char _asprotelum_character))
      (Utilities|IsValid _output_get
        (:Is%20Valid
          (bind _returnvalue (Ability|CommitAbility))
          (if _returnvalue
            (if (Ability|HasAuthority (Variables|Default|GetProtelum%20Char))
              (bind _returnvalue_2 (Class|ProtelumCharacter|GetProjectileSpawnTransform (Variables|Default|GetProtelum%20Char)))
              (bind _returnvalue_3 (Game|SpawnActorfromClass "/Game/AbilitySystem/GameplayAbilities/Shaman_Abilities/BP_Shaman_Projectile.BP_Shaman_Projectile_C" _returnvalue_2 "Undefined" (Variables|Default|GetProtelum%20Char) (Variables|Default|GetProtelum%20Char)))
              (bind _output_get_2 (Variables|Default|SetProjectile _returnvalue_3))
              (Utilities|IsValid _output_get_2
                (:Is%20Valid
                  (CallFunction|GetLevelParameters)
                  (Class|SimpleProjectile|ConfigureProjectile (Variables|Default|GetProjectile) "SingleTarget" (Variables|Default|GetInstigator%20Effects) (Variables|Default|GetTarget%20Effects) 0.0 (Variables|Default|GetProjectile%20Life%20Span) (Variables|Default|GetProjectile%20Color) (Math|Vector|MakeVector 1e+01 0.0 0.0) false)
                  (|WaitConfirmCancel
                    (:then
                      (EventDispatchers|AssignOnProjectileLifeEnds (Variables|Default|GetProjectile) (delegate Custom|OnProjectileLifeEnds_Event)))
                    (:OnConfirm
                      (Class|SimpleProjectile|ConfirmbyInstigator (Variables|Default|GetProjectile))
                      (Ability|EndAbility :!label _label))
                    (:OnCancel
                      (goto _label))))
                (:Is%20Not%20Valid
                  (Ability|CancelAbility))))
            (else
              (Ability|CancelAbility :!label _label_2))))
        (:Is%20Not%20Valid
          (goto _label_2))))
    (:CastFailed
      (goto _label_2))))

(event Ability|EventOnEndAbility
  (params (bWasCancelled :type Boolean)))

(fn SetTargetEffects
  (Variables|Default|SetTarget%20Effects (Utilities|Array|MakeArray (Ability|MakeOutgoingGameplayEffectSpec "/Game/AbilitySystem/GameplayAbilities/Shaman_Abilities/Shaman_SlowProjectileField/GE_Shaman_SlowField.GE_Shaman_SlowField_C" (Math|Conversions|ToFloat(Integer) (Ability|GetAbilityLevel)))))
  (return))

(fn GetLevelParameters
  (bind _outxy (DataTable|EvaluateCurveTableRow "/Game/AbilitySystem/GameplayAbilities/Shaman_Abilities/Shaman_SlowProjectileField/ShamanAbilityLevels_-_SlowProjectileField.ShamanAbilityLevels_-_SlowProjectileField" "ProjectileLifeSpan" (Math|Conversions|ToFloat(Integer) (Ability|GetAbilityLevel)))
    (:RowFound
      (Variables|Default|SetProjectile%20Life%20Span _outxy))
    (:RowNotFound
      _))
  (bind _outxy_2 (DataTable|EvaluateCurveTableRow "/Game/AbilitySystem/GameplayAbilities/Shaman_Abilities/Shaman_SlowProjectileField/ShamanAbilityLevels_-_SlowProjectileField.ShamanAbilityLevels_-_SlowProjectileField" "SlowFieldLifeSpan" (Math|Conversions|ToFloat(Integer) (Ability|GetAbilityLevel)))
    (:RowFound
      (Variables|Default|SetSlowFieldLifeSpan _outxy_2))
    (:RowNotFound
      _))
  (bind _outxy_3 (DataTable|EvaluateCurveTableRow "/Game/AbilitySystem/GameplayAbilities/Shaman_Abilities/Shaman_SlowProjectileField/ShamanAbilityLevels_-_SlowProjectileField.ShamanAbilityLevels_-_SlowProjectileField" "SlowStrenght" (Math|Conversions|ToFloat(Integer) (Ability|GetAbilityLevel)))
    (:RowFound
      (Variables|Default|SetSlowStrenght _outxy_3))
    (:RowNotFound
      _))
  (bind _outxy_4 (DataTable|EvaluateCurveTableRow "/Game/AbilitySystem/GameplayAbilities/Shaman_Abilities/Shaman_SlowProjectileField/ShamanAbilityLevels_-_SlowProjectileField.ShamanAbilityLevels_-_SlowProjectileField" "Diameter" (Math|Conversions|ToFloat(Integer) (Ability|GetAbilityLevel)))
    (:RowFound
      (Variables|Default|SetDiameter _outxy_4))
    (:RowNotFound
      _))
  (return))